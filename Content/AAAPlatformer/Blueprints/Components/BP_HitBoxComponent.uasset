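; BP_HitBoxComponent is an actor component that applies hit detection and damage from a bone or socket on the owner's skeletal mesh.
; OnStart clears the hit-actor list, and each OnTIck call sphere-traces at the given socket, ignoring already-hit actors so each is struck once per activation.
; A hit applies fixed damage, spawns an effect through the owner's BP_EffectComponent and plays a hit sound.
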(event EventBeginPlay
  (Private|Init))

(event EventTick
  (params (DeltaSeconds :type Float%20%28single-precision%29)))

(fn OnStart
  (Utilities|Array|Clear (Variables|Private|GetHitActors)))

(fn OnTIck
  (params (Bone :type Name))
  (bind _skeletalmeshcomponent (Variables|Private|GetSkeletalMeshComponent))
  (bind _returnvalue (Transformation|GetSocketLocation _skeletalmeshcomponent Bone))
  (bind (_outhit _returnvalue_2) (Collision|SphereTraceByChannel _returnvalue (+ _returnvalue "1.000000,1.000000,1.000000") (Variables|Property|GetRadius) (Variables|Property|GetTraceChannel) false (Variables|Private|GetHitActors) "ForOneFrame"))
  (if _returnvalue_2
    (Game|Damage|ApplyDamage (.HitActor (Collision|BreakHitResult _outhit)) 1e+02 0 (Variables|Private|GetOwner))
    (Utilities|Array|Add (Variables|Private|GetHitActors) (.HitActor (Collision|BreakHitResult _outhit)))
    (Default|Spawn (Variables|Private|GetEffectComponent) "NewEnumerator4" (.Location (Collision|BreakHitResult _outhit)))
    (Audio|PlaySound2D "/Game/AAAPlatformer/Sounds/Hit/SC_Hit.SC_Hit" 1.0 1.0 0.0 0 0)))

(fn Init
  (Variables|Private|SetOwner (Components|GetOwner))
  (Variables|Private|SetSkeletalMeshComponent (Actor|GetComponentbyClass (Variables|Private|GetOwner) "/Script/Engine.SkeletalMeshComponent"))
  (Variables|Private|SetEffectComponent (Actor|GetComponentbyClass (Variables|Private|GetOwner) "/Game/AAAPlatformer/Blueprints/Components/BP_EffectComponent.BP_EffectComponent_C")))