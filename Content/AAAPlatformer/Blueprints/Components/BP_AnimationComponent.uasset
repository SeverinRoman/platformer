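; BP_AnimationComponent is a component that plays animation montages on its owning actor by animation type.
; On BeginPlay it caches the owner, the AnimInstance of the owner's skeletal mesh and the owner's BP_StateComponent.
; Play looks up the requested type in the Animations map and plays the matching montage if the AnimInstance is valid.
; The state component is otherwise unused, as its only SetState call is disconnected.
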(event EventBeginPlay
  (Private|Init))

(event EventTick
  (params (DeltaSeconds :type Float%20%28single-precision%29)))

(fn Play
  (params (AnimationType :type E_AnimationType%20Enum :default "NewEnumerator0"))
  (bind _animinstance (Variables|Private|GetAnimInstance))
  (if (Utilities|Map|Contains (Variables|Public|GetAnimations) AnimationType)
    (Utilities|IsValid _animinstance
      (:Is%20Valid
        (Animation|Montage|MontagePlay _animinstance (.Value (Utilities|Map|Find (Variables|Public|GetAnimations) AnimationType)) 1.0 "MontageLength" 0.0 true)))))

(fn Init
  (bind _output_get (Variables|Private|SetOwner (Components|GetOwner)))
  (Variables|Private|SetAnimInstance (Components|SkeletalMesh|GetAnimInstance (Actor|GetComponentbyClass _output_get "/Script/Engine.SkeletalMeshComponent")))
  (Variables|Private|SetStateComponent (Actor|GetComponentbyClass (Variables|Private|GetOwner) "/Game/AAAPlatformer/Blueprints/Components/BP_StateComponent.BP_StateComponent_C")))