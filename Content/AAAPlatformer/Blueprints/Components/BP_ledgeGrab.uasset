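; Ledge-grab component that detects and measures walls in front of its owner; it does not yet perform a grab.
; It caches the owner's BP_StateComponent and, each Tick in one specific state, line-traces forward for a wall.
; On a hit, a second downward trace from above the impact point finds the wall top.
; The height difference between the two hits is stored and printed for debugging.
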(event EventBeginPlay
  (Private|Init))

(event EventTick
  (params (DeltaSeconds :type Float%20%28single-precision%29))
  (bind _owner (Variables|Private|GetOwner))
  (bind _returnvalue (Transformation|GetActorLocation _owner))
  (Utilities|IsValid (Variables|Private|GetStateComponent)
    (:Is%20Valid
      (if (Utilities|Enum|Equal(Enum) (Default|GetState (Variables|Private|GetStateComponent)) "NewEnumerator3")
        (Utilities|IsValid (Variables|Private|GetOwner)
          (:Is%20Valid
            (bind (_outhit _returnvalue_2) (Collision|LineTraceByChannel _returnvalue (+ _returnvalue (* (Transformation|GetActorForwardVector _owner) (Variables|Property|GetDistance))) "TraceTypeQuery1" false 0 (Variables|Property|GetDrawDebugType)))
            (if _returnvalue_2
              (Variables|Private|SetWallLocation (.Location (Collision|BreakHitResult _outhit)))
              (Variables|Private|SetWallNormalLocation (.Normal (Collision|BreakHitResult _outhit)))
              (bind (_outhit_2 _returnvalue_3) (Collision|LineTraceByChannel (+ "0, 0,300.000000" (+ (Variables|Private|GetWallLocation) (* (Math|Vector|GetForwardVector (Math|Rotator|MakeRotfromX (Variables|Private|GetWallNormalLocation))) 0.0))) (- (+ "0, 0,300.000000" (+ (Variables|Private|GetWallLocation) (* (Math|Vector|GetForwardVector (Math|Rotator|MakeRotfromX (Variables|Private|GetWallNormalLocation))) 0.0))) "0, 0,300.000000") "TraceTypeQuery1" false 0 (Variables|Property|GetDrawDebugType)))
              (if _returnvalue_3
                (Variables|Private|SetWallHeightLocation (.Location (Collision|BreakHitResult _outhit_2)))
                (bind _output_get (Variables|Private|SetWallheight (.Z (Math|Vector|BreakVector (- (Variables|Private|GetWallHeightLocation) (Variables|Private|GetWallLocation))))))
                (Development|PrintString (Utilities|String|ToString(Float) _output_get))))))))))

(fn Init
  (bind _output_get (Variables|Private|SetOwner (Components|GetOwner)))
  (Utilities|IsValid _output_get
    (:Is%20Valid
      (Variables|Private|SetStateComponent (Actor|GetComponentbyClass _output_get "/Game/AAAPlatformer/Blueprints/Components/BP_StateComponent.BP_StateComponent_C")))))