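; Actor component that tracks its owner's locomotion state in the platformer.
; Caches the owner's CharacterMovementComponent on BeginPlay, then samples velocity, speed and falling status each tick to derive the state enum.
; Falling overrides any state, while on the ground only the three locomotion states switch between stationary and moving, leaving others set through SetState intact.
; An optional debug flag prints the current state every tick.
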(event EventBeginPlay
  (Private|Init))

(event EventTick
  (params (DeltaSeconds :type Float%20%28single-precision%29))
  (Utilities|IsValid (Variables|Private|GetOwner)
    (:Is%20Valid
      (Utilities|IsValid (Variables|Default|GetCharacterMoveComponent)
        (:Is%20Valid
          (Utilities|FlowControl|Sequence
            (:then_0
              (Private|Update))
            (:then_1
              (Private|UpdateState))
            (:then_2
              (if (Variables|Public|GetIsDebug)
                (Development|PrintString (Utilities|String|EnumtoString (Variables|Private|GetState)) true true "(R=0.000000,G=1.000000,B=0.000000,A=1.000000)" 0.001)))))))))

(fn Init
  (bind _output_get (Variables|Private|SetOwner (Components|GetOwner)))
  (Utilities|IsValid _output_get
    (:Is%20Valid
      (Variables|Default|SetCharacterMoveComponent (Actor|GetComponentbyClass (Variables|Private|GetOwner) "/Script/Engine.CharacterMovementComponent")))))

(fn Update
  (Utilities|IsValid (Variables|Default|GetCharacterMoveComponent)
    (:Is%20Valid
      (bind _output_get (Variables|Private|SetVelocity (Variables|/Script/Engine.MovementComponent|GetVelocity (Variables|Default|GetCharacterMoveComponent))))
      (Variables|Private|SetSpeed (Math|Vector|VectorLength _output_get))
      (Variables|Private|SetIsFalling (AI|Components|NavMovement|IsFalling (Variables|Default|GetCharacterMoveComponent))))))

(fn GetState
  (return (Variables|Private|GetState)))

(fn SetState
  (params (NewState :type E_StateType%20Enum :default "NewEnumerator0"))
  (if (!= NewState (Variables|Private|GetState))
    (Variables|Private|SetState NewState)))

(fn UpdateState
  (bind _state (Variables|Private|GetState))
  (if (Variables|Private|GetIsFalling)
    (Private|SetState "NewEnumerator3")
    (elif (Math|Boolean|ORBoolean (Utilities|Enum|Equal(Enum) _state "NewEnumerator1") (Utilities|Enum|Equal(Enum) _state "NewEnumerator2") (Utilities|Enum|Equal(Enum) _state "NewEnumerator3"))
      (if (> (Variables|Private|GetSpeed) 0.0)
        (Private|SetState "NewEnumerator2")
        (else
          (Private|SetState "NewEnumerator1"))))))