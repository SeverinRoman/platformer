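; BP_ShadowComponent is a component that keeps a static mesh on the surface beneath its owner, apparently as a drop shadow.
; SetStaticMesh supplies the mesh to move.
; Each tick, a Visibility line trace runs from the owner, with its end Z computed by scaling world height by a negative factor rather than subtracting a fixed distance.
; On a hit, the mesh teleports to the impact location plus an offset.
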(event EventTick
  (params (DeltaSeconds :type Float%20%28single-precision%29))
  (bind _owner (Variables|Private|GetOwner))
  (bind _returnvalue (Transformation|GetActorLocation _owner))
  (bind _returnvalue_2 (Transformation|GetActorUpVector _owner))
  (bind _returnvalue_3 (+ _returnvalue _returnvalue_2))
  (Utilities|IsValid (Variables|Default|GetStaticMeshComponent)
    (:Is%20Valid
      (Utilities|IsValid (Variables|Private|GetOwner)
        (:Is%20Valid
          (bind (_outhit _returnvalue_4) (Collision|LineTraceByChannel _returnvalue (Math|Vector|MakeVector (.x _returnvalue_3) (.y _returnvalue_3) (* (.z _returnvalue_3) -1e+02)) "TraceTypeQuery1" false 0 (Variables|Private|GetDrawDebugType)))
          (if _returnvalue_4
            (Transformation|SetWorldLocation (Variables|Default|GetStaticMeshComponent) (+ (.Location (Collision|BreakHitResult _outhit)) (Variables|Private|GetOffset)) false true)))))))

(event EventBeginPlay
  (Variables|Private|SetOwner (Components|GetOwner)))

(fn SetStaticMesh
  (params (NewStaticMesh :type Static%20Mesh%20Component%20Object%20Reference))
  (Variables|Default|SetStaticMeshComponent NewStaticMesh))