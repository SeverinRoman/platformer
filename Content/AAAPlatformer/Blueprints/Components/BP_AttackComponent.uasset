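; BP_AttackComponent is an actor component that runs its owner's attack, alternating left and right animations with simple combo chaining.
; It caches the owner's state and animation components, then attacks only when the state is not busy, setting the attack state and blending in the upper body.
; An attack requested during another sets a combo flag, which OnCombo consumes to reset the state and attack again.
; OnAttackEnd resets the state and upper-body blend.
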(event EventBeginPlay
  (Private|Init))

(event EventTick
  (params (DeltaSeconds :type Float%20%28single-precision%29)))

(fn Attack
  (Private|Combo)
  (if (not (Private|GetIsBusy))
    (Default|SetState (Variables|Components|GetStateComponent) "NewEnumerator6")
    (Default|BlendUpBody (Variables|Components|GetAnimationComponent) true)
    (if (Variables|Private|GetIsAttackLeft)
      (Default|Play (Variables|Components|GetAnimationComponent) "NewEnumerator4")
      (Variables|Private|SetIsAttackLeft false)
      (else
        (Default|Play (Variables|Components|GetAnimationComponent) "NewEnumerator5")
        (Variables|Private|SetIsAttackLeft true)))))

(fn OnCombo
  (if (Variables|Private|GetIsCombo)
    (Variables|Private|SetIsCombo false)
    (Default|SetState (Variables|Components|GetStateComponent) "NewEnumerator1")
    (Public|Attack)))

(fn Init
  (LocalVariables|SetOwner (Components|GetOwner))
  (Utilities|FlowControl|Sequence
    (:then_0
      (Variables|Components|SetStateComponent (Actor|GetComponentbyClass (LocalVariables|GetOwner) "/Game/AAAPlatformer/Blueprints/Components/BP_StateComponent.BP_StateComponent_C")))
    (:then_1
      (Variables|Components|SetAnimationComponent (Actor|GetComponentbyClass (LocalVariables|GetOwner) "/Game/AAAPlatformer/Blueprints/Components/BP_AnimationComponent.BP_AnimationComponent_C")))))

(fn GetIsBusy
  (bind _statecomponent (Variables|Components|GetStateComponent))
  (bind _statetype (Default|GetState _statecomponent))
  (if (and (Utilities|Enum|NotEqual(Enum) _statetype "NewEnumerator1") (Utilities|Enum|NotEqual(Enum) _statetype "NewEnumerator2"))
    (return true)
    (else
      (return false))))

(fn OnAttackEnd
  (Default|SetState (Variables|Components|GetStateComponent) "NewEnumerator1")
  (Default|BlendUpBody (Variables|Components|GetAnimationComponent) false))

(fn Combo
  (Variables|Private|SetIsCombo (Utilities|Enum|Equal(Enum) "NewEnumerator6" (Default|GetState (Variables|Components|GetStateComponent)))))