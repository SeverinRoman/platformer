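; BP_DeadComponent is an actor component that handles the death of its owner.
; On BeginPlay it caches the owner's state, ragdoll and capsule components.
; Its Dead function triggers the ragdoll component and switches the capsule to the "Dead" collision profile.
; The state component is cached but not used here, and nothing in this Blueprint calls Dead.
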(event EventBeginPlay
  (Private|Init))

(fn Dead
  (Default|Ragdoll (Variables|Default|GetRagdollComponent))
  (Collision|SetCollisionProfileName (Variables|Default|GetCapsuleComponent) "Dead" :!class /Script/Engine.PrimitiveComponent))

(fn Init
  (Variables|Default|SetOwner (Components|GetOwner))
  (Variables|Default|SetStateComponent (Actor|GetComponentbyClass (Variables|Default|GetOwner) "/Game/AAAPlatformer/Blueprints/Components/BP_StateComponent.BP_StateComponent_C"))
  (Variables|Default|SetRagdollComponent (Actor|GetComponentbyClass (Variables|Default|GetOwner) "/Game/AAAPlatformer/Blueprints/Components/BP_RagdollComponent.BP_RagdollComponent_C"))
  (Variables|Default|SetCapsuleComponent (Actor|GetComponentbyClass (Variables|Default|GetOwner) "/Script/Engine.CapsuleComponent")))