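; BP_EffectComponent is an actor component that spawns particle effects for its owner, including footstep effects at each leg.
; On BeginPlay it caches the owner and its skeletal mesh component.
; Spawn looks up an emitter template in an Effects map by effect type and plays it at a given location.
; LeftStep and RightStep call Spawn with one shared effect type at the left or right leg socket.
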(event EventBeginPlay
  (Private|Init))

(event EventTick
  (params (DeltaSeconds :type Float%20%28single-precision%29)))

(fn Spawn
  (params (EffectType :type E_EffectType%20Enum :default "NewEnumerator0") (Location :type Vector))
  (if (Utilities|Map|Contains (Variables|Public|GetEffects) EffectType)
    (Effects|SpawnEmitteratLocation (.Value (Utilities|Map|Find (Variables|Public|GetEffects) EffectType)) Location)))

(fn LeftStep
  (bind _skeletalmeshcomponent (Variables|Default|GetSkeletalMeshComponent))
  (Utilities|IsValid _skeletalmeshcomponent
    (:Is%20Valid
      (Public|Spawn "NewEnumerator1" (Transformation|GetSocketLocation _skeletalmeshcomponent (Variables|Public|GetLeftLeg))))))

(fn Init
  (bind _output_get (Variables|Private|SetOwner (Components|GetOwner)))
  (Variables|Default|SetSkeletalMeshComponent (Actor|GetComponentbyClass _output_get "/Script/Engine.SkeletalMeshComponent")))

(fn RightStep
  (bind _skeletalmeshcomponent (Variables|Default|GetSkeletalMeshComponent))
  (Utilities|IsValid _skeletalmeshcomponent
    (:Is%20Valid
      (Public|Spawn "NewEnumerator1" (Transformation|GetSocketLocation _skeletalmeshcomponent (Variables|Public|GetRightLeg))))))