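; BP_RagdollComponent is an actor component that switches its owner into physics-driven ragdoll.
; On BeginPlay it caches the owning pawn, its skeletal mesh and its BP_StateComponent.
; Its Ragdoll function sets a state on the state component, then turns on physics simulation for the mesh, with no recovery path in the component.
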(event EventBeginPlay
  (Private|Init))

(fn Init
  (bind _returnvalue (Components|GetOwner))
  (Variables|Private|SetPawn _returnvalue)
  (Variables|Private|SetSkeletalMesh (Actor|GetComponentbyClass _returnvalue "/Script/Engine.SkeletalMeshComponent"))
  (Variables|Private|SetStateComponent (Actor|GetComponentbyClass _returnvalue "/Game/AAAPlatformer/Blueprints/Components/BP_StateComponent.BP_StateComponent_C")))

(fn Ragdoll
  (Default|SetState (Variables|Private|GetStateComponent) "NewEnumerator4")
  (Physics|SetSimulatePhysics (Variables|Private|GetSkeletalMesh) true))